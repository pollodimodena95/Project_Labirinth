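; Game mode for the maze game that manages the HUD and the win and lose end states.
; BeginPlay creates and displays the heads-up display widget.
; The Win and Lose events disable player input, fade the camera to near-white or red, and remove the HUD.
; After a short delay each shows its end screen widget with the mouse cursor and UI-only input.
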(event Custom|Lose
  (bind _returnvalue (Game|GetPlayerController 0))
  (Input|DisableInput (Game|GetPlayerCharacter 0) (Game|GetPlayerController 0))
  (CameraFades|StartCameraFade (Game|GetPlayerCameraManager 0) 0.0 0.8 2.0 "(R=1.000000,G=0.000000,B=0.026276,A=1.000000)" false true)
  (Widget|RemovefromParent (Variables|Default|GetHeadsUpDisplay))
  (Utilities|FlowControl|Delay 2.0)
  (bind _returnvalue_2 (UserInterface|CreateWidget "/Game/UI/WB_LoseScreen.WB_LoseScreen_C"))
  (UserInterface|Viewport|AddtoViewport _returnvalue_2 0)
  (Variables|/Script/Engine.PlayerController|SetbShowMouseCursor _returnvalue true)
  (Input|SetInputModeUIOnly _returnvalue _returnvalue_2 "DoNotLock"))

(event Custom|Win
  (bind _returnvalue (Game|GetPlayerController 0))
  (Input|DisableInput (Game|GetPlayerCharacter 0) (Game|GetPlayerController 0))
  (CameraFades|StartCameraFade (Game|GetPlayerCameraManager 0) 0.0 0.8 2.0 "(R=0.976708,G=0.989687,B=1.000000,A=1.000000)" false true)
  (Widget|RemovefromParent (Variables|Default|GetHeadsUpDisplay))
  (Utilities|FlowControl|Delay 2.0)
  (bind _returnvalue_2 (UserInterface|CreateWidget "/Game/UI/WB_WinScreen.WB_WinScreen_C"))
  (UserInterface|Viewport|AddtoViewport _returnvalue_2 0)
  (Variables|/Script/Engine.PlayerController|SetbShowMouseCursor _returnvalue true)
  (Input|SetInputModeUIOnly _returnvalue 0 "DoNotLock"))

(event EventBeginPlay
  (bind _returnvalue (UserInterface|CreateWidget "/Game/UI/WB_HeadsUpDisplay.WB_HeadsUpDisplay_C"))
  (bind _output_get (Variables|Default|SetHeadsUpDisplay _returnvalue))
  (UserInterface|Viewport|AddtoViewport _output_get 0))

(event EventTick
  (params (DeltaSeconds :type Float%20%28single-precision%29)))

(fn ConstructionScript)