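; Base weapon actor that fires arrow projectiles and tracks clip and reserve ammo, working as a child actor of the player character.
; StartShooting and StopShooting only toggle IsFiring.
; FireBullet spawns BP_arrow at the barrel along the camera's rotation, passing speed and gravity, then decrements ammo and plays a sound at the player.
; Reload refills the clip from the reserve, taking whatever remains when short.
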(event Custom|Start%20Shooting
  (Variables|Default|SetIs%20Firing true))

(event Custom|Stop%20Shooting
  (Variables|Default|SetIs%20Firing false))

(event EventBeginPlay)

(fn ConstructionScript)

(fn FireBullet
  (bind _asplayer_character_bp (Utilities|Casting|CastToPlayer_Character_BP (Actor|GetParentActor)))
  (if (> (Variables|Default|GetAmmo%20Current) 0)
    (Game|SpawnActorfromClass "/Game/BP/BP_arrow.BP_arrow_C" (Math|Transform|MakeTransform (Transformation|GetWorldLocation (Variables|Default|GetBarrel%20Ref)) (Transformation|GetWorldRotation (Variables|/Game/Game/Player_Character_BP.Player_Character_BP_C|GetCamera _asplayer_character_bp))) "AdjustIfPossibleButDontSpawnIfColliding" 0 (Variables|Default|GetBullet%20Speed) (Variables|Default|GetGravity) 0)
    (Math|Integer|DecrementInt (Variables|Default|GetAmmo%20Current)
      (:%20%20
        (Audio|PlaySoundatLocation "/Game/Sounds/Arrow_SFX.Arrow_SFX" (Transformation|GetActorLocation (Game|GetPlayerCharacter 0)) "0, 0, 0" 1.0 1.0 0.0 0 0 0)))))

(fn Reload
  (bind _output_get (LocalVariables|SetBullet%20Difference (- (Variables|Default|GetClip%20Size) (Variables|Default|GetAmmo%20Current))))
  (if (>= (Variables|Default|GetAmmo%20Max) _output_get)
    (Variables|Default|SetAmmo%20Current (Variables|Default|GetClip%20Size))
    (Variables|Default|SetAmmo%20Max (- (Variables|Default|GetAmmo%20Max) (LocalVariables|GetBullet%20Difference)))
    (else
      (Variables|Default|SetAmmo%20Current (+ (Variables|Default|GetAmmo%20Current) (Variables|Default|GetAmmo%20Max)))
      (Variables|Default|SetAmmo%20Max 0))))