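; First-person-style player character for the maze game mode, handling movement, health and weapon input.
; Camera-relative movement shares a DoOnce that throttles footstep sounds to half-second intervals, and look axes drive controller yaw and pitch.
; Damage lowers Health, refreshes the HUD through the cached Gm_Maze and triggers its Lose at zero.
; Fire (Spara) and reload inputs forward to the Weapon_Parent_BP held in the Weapon child actor component.
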(event Game|Damage|EventAnyDamage
  (params (Damage :type Float%20%28single-precision%29) (DamageType :type Damage%20Type%20Object%20Reference) (InstigatedBy :type Controller%20Object%20Reference) (DamageCauser :type Actor%20Object%20Reference))
  (bind _gamemode (Variables|Default|GetGameMode))
  (Variables|Default|SetHealth (- (Variables|Default|GetHealth) (Math|Float|Truncate Damage)))
  (Default|UpdateHealth (Variables|/Game/Game/Game/GM_Maze.Gm_Maze_C|GetHeadsUpDisplay _gamemode))
  (if (<= (Variables|Default|GetHealth) 0)
    (Default|Lose _gamemode)))

(event EventBeginPlay
  (bind _asgm_maze (Utilities|Casting|CastToGm_Maze (Game|GetGameMode)))
  (Variables|Default|SetGameMode _asgm_maze))

(event Input|ActionEvents|InputActionSpara
  (params (Key :type Key%20Structure :default "None"))
  (:Pressed
    (bind _asweapon_parent_bp (Utilities|Casting|CastToWeapon_Parent_BP (Variables|/Script/Engine.ChildActorComponent|GetChildActor (Variables|Default|GetWeapon))))
    (Default|StartShooting _asweapon_parent_bp))
  (:Released
    (Default|StopShooting _asweapon_parent_bp)))

(event Input|ActionEvents|InputActionReload
  (params (Key :type Key%20Structure :default "None"))
  (:Pressed
    (bind _asweapon_parent_bp (Utilities|Casting|CastToWeapon_Parent_BP (Variables|/Script/Engine.ChildActorComponent|GetChildActor (Variables|Default|GetWeapon))))
    (Default|Reload _asweapon_parent_bp)))

(event Input|AxisEvents|InputAxisMoveForward
  (params (AxisValue :type Float%20%28single-precision%29))
  (Pawn|Input|AddMovementInput (Math|Vector|GetForwardVector (Transformation|GetWorldRotation (Variables|Default|GetCamera))) AxisValue false)
  (if (!= AxisValue 0.0)
    (Utilities|FlowControl|DoOnce false :!label _label
      (:Completed
        (Audio|PlaySoundatLocation "/Game/Sounds/Footstep_SFX.Footstep_SFX" (Transformation|GetActorLocation) "0, 0, 0" 1.0 1.0 0.0 0 0 0)
        (Utilities|FlowControl|Delay 0.5)
        (goto _label Reset)))))

(event Input|AxisEvents|InputAxisMoveRight
  (params (AxisValue :type Float%20%28single-precision%29))
  (Pawn|Input|AddMovementInput (Math|Vector|GetRightVector (Transformation|GetWorldRotation (Variables|Default|GetCamera))) AxisValue false)
  (if (!= AxisValue 0.0)
    (Utilities|FlowControl|DoOnce false :!label _label
      (:Completed
        (Audio|PlaySoundatLocation "/Game/Sounds/Footstep_SFX.Footstep_SFX" (Transformation|GetActorLocation) "0, 0, 0" 1.0 1.0 0.0 0 0 0)
        (Utilities|FlowControl|Delay 0.5)
        (goto _label Reset)))))

(event Input|AxisEvents|InputAxisLookup
  (params (AxisValue :type Float%20%28single-precision%29))
  (Pawn|Input|AddControllerPitchInput AxisValue))

(event Input|AxisEvents|InputAxisTurn
  (params (AxisValue :type Float%20%28single-precision%29))
  (Pawn|Input|AddControllerYawInput AxisValue))

(fn ConstructionScript)