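; Bow weapon, child of a base weapon, that charges while shooting and scales projectile speed by the charge.
; A timeline paced by ChargeTime drives CurrentCharge while the charge widget from the Gm_Maze HUD is visible.
; Stopping, or reaching full charge, fires if minimally charged, then hides the widget and reverses the timeline.
; A new draw requires ammo and a mostly drained charge.
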(event EventFireBullet
  (Variables|Default|SetBullet%20Speed (* (Variables|Default|GetBullet%20Speed) (Variables|Default|GetCurrent%20Charge)))
  (|CallParentFunction)
  (Variables|Default|SetBullet%20Speed 3e+03))

(event EventStartShooting
  (|CallParentFunction)
  (if (Math|Boolean|ANDBoolean (not (Variables|Default|GetIsCharging?)) (<= (Variables|Default|GetCurrent%20Charge) 0.2) (> (Variables|Default|GetAmmo%20Current) 0))
    (Widget|SetVisibility (Variables|Default|GetCharge%20UI) "Visible")
    (Variables|Default|SetIsCharging? true)
    (Components|Timeline|SetPlayRate (Variables|Default|GetCharge%20Weapon) (/ 1.0 (Variables|Default|GetCharge%20Time)))
    (bind _weapon_charge (Timeline|Charge%20Weapon Play)
      (:Update
        (bind _output_get (Variables|Default|SetCurrent%20Charge (Math|Float|Clamp(Float) _weapon_charge)))
        (if (>= _output_get 1.0)
          (CallFunction|StopShooting))))))

(event EventStopShooting
  (|CallParentFunction)
  (Widget|SetVisibility (Variables|Default|GetCharge%20UI) "Hidden")
  (if (and (Variables|Default|GetIsCharging?) (>= (Variables|Default|GetCurrent%20Charge) 0.1))
    (CallFunction|FireBullet))
  (Variables|Default|SetIsCharging? false)
  (Components|Timeline|SetPlayRate (Variables|Default|GetCharge%20Weapon) 1.0)
  (bind _weapon_charge (Timeline|Charge%20Weapon Reverse)
    (:Update
      (bind _output_get (Variables|Default|SetCurrent%20Charge (Math|Float|Clamp(Float) _weapon_charge)))
      (if (>= _output_get 1.0)
        (CallFunction|StopShooting)))))

(event EventBeginPlay
  (bind _asgm_maze (Utilities|Casting|CastToGm_Maze (Game|GetGameMode)))
  (bind _output_get (Variables|Default|SetCharge%20UI (Variables|/Game/UI/WB_HeadsUpDisplay.WB_HeadsUpDisplay_C|GetWB_Charge_UI (Variables|/Game/Game/Game/GM_Maze.Gm_Maze_C|GetHeadsUpDisplay _asgm_maze))))
  (Widget|SetVisibility _output_get "Hidden"))

(fn ConstructionScript
  (|CallParentFunction))