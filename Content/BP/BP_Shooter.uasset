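; BP_Shooter is a trap-like actor that fires arrows when the player crosses its line of sight.
; Each Tick it sphere-traces 3000 units forward from ArrowSource on the Camera channel.
; While the player character is hit, ShootArrow runs every frame without cooldown, spawning BP_arrow at ArrowSource and playing a sound at the player's location.
; A looping timer for ShootArrow exists but is never executed.
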(event Custom|Shoot%20Arrow
  (Game|SpawnActorfromClass "/Game/BP/BP_arrow.BP_arrow_C" (Transformation|GetWorldTransform (Variables|Default|GetArrow%20Source)) "Undefined" 0 0)
  (Audio|PlaySoundatLocation "/Game/Sounds/Arrow_SFX.Arrow_SFX" (Transformation|GetActorLocation (Game|GetPlayerCharacter 0)) "0, 0, 0" 1.0 1.0 0.0 0 0 0))

(event EventBeginPlay)

(event EventTick
  (params (DeltaSeconds :type Float%20%28single-precision%29))
  (bind _arrow_source (Variables|Default|GetArrow%20Source))
  (bind _returnvalue (Transformation|GetWorldLocation _arrow_source))
  (bind _outhit (Collision|SphereTraceByChannel _returnvalue (+ _returnvalue (* (Math|Vector|GetForwardVector (Transformation|GetWorldRotation _arrow_source)) 3000)) 0.0 "TraceTypeQuery2" false 0 "None"))
  (if (== (.hitactor _outhit) (Game|GetPlayerCharacter 0))
    (CallFunction|ShootArrow)))

(fn ConstructionScript)