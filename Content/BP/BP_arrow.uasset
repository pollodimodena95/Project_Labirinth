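; BP_arrow is a projectile arrow that damages and knocks back the player character on overlap.
; The construction script applies the BulletSpeed and ProjectileGravity variables to its ProjectileMovement component.
; When ArrowCollision overlaps a Player_Character_BP with health remaining, it launches the character with the arrow's velocity, applies damage, destroys itself and plays a hit sound at the player's location.
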(event OnComponentBeginOverlap(ArrowCollision)
  (params (OverlappedComponent :type Primitive%20Component%20Object%20Reference) (OtherActor :type Actor%20Object%20Reference) (OtherComp :type Primitive%20Component%20Object%20Reference) (OtherBodyIndex :type Integer) (bFromSweep :type Boolean) (SweepResult :type Hit%20Result%20Structure%20%28by%20ref%29))
  (bind _asplayer_character_bp (Utilities|Casting|CastToPlayer_Character_BP OtherActor))
  (if (> (Variables|/Game/Game/Player_Character_BP.Player_Character_BP_C|GetHealth _asplayer_character_bp) 0)
    (Character|LaunchCharacter _asplayer_character_bp (+ (Transformation|GetVelocity) "0, 0, 0") false false)
    (Game|Damage|ApplyDamage _asplayer_character_bp 1.0 (Game|GetPlayerController 0) 0)
    (Actor|DestroyActor)
    (Audio|PlaySoundatLocation "/Game/Sounds/Hit_SFX.Hit_SFX" (Transformation|GetActorLocation (Game|GetPlayerCharacter 0)) "0, 0, 0" 1.0 1.0 0.0 0 0 0)))

(fn ConstructionScript
  (bind _projectilemovement (Variables|Default|GetProjectileMovement))
  (bind _bullet_speed (Variables|Default|GetBullet%20Speed))
  (Variables|/Script/Engine.ProjectileMovementComponent|SetInitialSpeed _projectilemovement _bullet_speed)
  (Variables|/Script/Engine.ProjectileMovementComponent|SetMaxSpeed _projectilemovement _bullet_speed)
  (Variables|/Script/Engine.ProjectileMovementComponent|SetProjectileGravityScale (Variables|Default|GetProjectileMovement) (Variables|Default|GetProjectile%20gravity)))