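; Maze door that the player opens by spending a key, shown to the player as a Golden Skull.
; Its trigger volume toggles actor input by key count and shows prompts through the Gm_Maze game mode's HUD.
; Interact decrements the key count, refreshes the skull display and spawns a key mesh snapped to the keyhole.
; A timeline then moves key and door with sound, marking the door open and clearing the message when finished.
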(event OnComponentBeginOverlap(Trigger_Volume)
  (params (OverlappedComponent :type Primitive%20Component%20Object%20Reference) (OtherActor :type Actor%20Object%20Reference) (OtherComp :type Primitive%20Component%20Object%20Reference) (OtherBodyIndex :type Integer) (bFromSweep :type Boolean) (SweepResult :type Hit%20Result%20Structure%20%28by%20ref%29))
  (if (== OtherActor (Game|GetPlayerCharacter 0))
    (bind _asgm_maze (Utilities|Casting|CastToGm_Maze (Game|GetGameMode)))
    (if (not (Variables|Default|GetIsOpen?))
      (bind _asplayer_character_bp (Utilities|Casting|CastToPlayer_Character_BP (Game|GetPlayerCharacter 0)))
      (if (> (Variables|/Game/Game/Player_Character_BP.Player_Character_BP_C|GetNumber%20of%20Keys _asplayer_character_bp) 0)
        (Input|EnableInput (Game|GetPlayerController 0))
        (Variables|/Game/UI/WB_HeadsUpDisplay.WB_HeadsUpDisplay_C|SetMessage (Variables|/Game/Game/Game/GM_Maze.Gm_Maze_C|GetHeadsUpDisplay _asgm_maze) "Press E to Open Door")
        (Default|UpdateMessage (Variables|/Game/Game/Game/GM_Maze.Gm_Maze_C|GetHeadsUpDisplay _asgm_maze))
        (else
          (Input|DisableInput (Game|GetPlayerController 0))
          (bind _asgm_maze_2 (Utilities|Casting|CastToGm_Maze (Game|GetGameMode)))
          (Variables|/Game/UI/WB_HeadsUpDisplay.WB_HeadsUpDisplay_C|SetMessage (Variables|/Game/Game/Game/GM_Maze.Gm_Maze_C|GetHeadsUpDisplay _asgm_maze_2) "Door Requires Golden Skull")
          (Default|UpdateMessage (Variables|/Game/Game/Game/GM_Maze.Gm_Maze_C|GetHeadsUpDisplay _asgm_maze_2)))))))

(event OnComponentEndOverlap(Trigger_Volume)
  (params (OverlappedComponent :type Primitive%20Component%20Object%20Reference) (OtherActor :type Actor%20Object%20Reference) (OtherComp :type Primitive%20Component%20Object%20Reference) (OtherBodyIndex :type Integer))
  (if (== OtherActor (Game|GetPlayerCharacter 0))
    (Input|DisableInput (Game|GetPlayerController 0))
    (bind _asgm_maze (Utilities|Casting|CastToGm_Maze (Game|GetGameMode)))
    (Variables|/Game/UI/WB_HeadsUpDisplay.WB_HeadsUpDisplay_C|SetMessage (Variables|/Game/Game/Game/GM_Maze.Gm_Maze_C|GetHeadsUpDisplay _asgm_maze) "")
    (Default|UpdateMessage (Variables|/Game/Game/Game/GM_Maze.Gm_Maze_C|GetHeadsUpDisplay _asgm_maze))))

(event Input|ActionEvents|InputActionInteract
  (params (Key :type Key%20Structure :default "None"))
  (:Pressed
    (bind _asplayer_character_bp (Utilities|Casting|CastToPlayer_Character_BP (Game|GetPlayerCharacter 0)))
    (if (> (Variables|/Game/Game/Player_Character_BP.Player_Character_BP_C|GetNumber%20of%20Keys _asplayer_character_bp) 0)
      (Math|Integer|DecrementInt (Variables|/Game/Game/Player_Character_BP.Player_Character_BP_C|GetNumber%20of%20Keys _asplayer_character_bp)
        (:%20%20
          (bind _asgm_maze (Utilities|Casting|CastToGm_Maze (Game|GetGameMode)))
          (Default|UpdateSkulls (Variables|/Game/Game/Game/GM_Maze.Gm_Maze_C|GetHeadsUpDisplay _asgm_maze))
          (bind _returnvalue (AddComponent|AddStaticMeshComponent false))
          (bind _output_get (Variables|Default|SetKey%20Mesh _returnvalue))
          (Transformation|AttachComponentToComponent _output_get (Variables|Default|Getkeyhole) "None" "SnapToTarget" "SnapToTarget" "SnapToTarget" true)
          (Audio|PlaySoundatLocation "/Game/Sounds/DoorOpening_SFX.DoorOpening_SFX" (Transformation|GetActorLocation) "0, 0, 0" 1.0 1.0 0.0 0 0 0)
          (bind (_direction _door_pos _key_pos) (Timeline|Door%20Opening PlayFromStart)
            (:Update
              (Transformation|SetRelativeLocation (Variables|Default|GetKey%20Mesh) (Math|Vector|MakeVector 0.0 _key_pos 0.0) false false)
              (Transformation|SetRelativeLocation (Variables|Default|GetDoor%20Mesh) (Math|Vector|MakeVector 0.0 0.0 _door_pos) false false))
            (:Finished
              (Variables|Default|SetIsOpen? true)
              (bind _asgm_maze_2 (Utilities|Casting|CastToGm_Maze (Game|GetGameMode)))
              (Variables|/Game/UI/WB_HeadsUpDisplay.WB_HeadsUpDisplay_C|SetMessage (Variables|/Game/Game/Game/GM_Maze.Gm_Maze_C|GetHeadsUpDisplay _asgm_maze_2) "")
              (Default|UpdateMessage (Variables|/Game/Game/Game/GM_Maze.Gm_Maze_C|GetHeadsUpDisplay _asgm_maze_2)))))))))

(fn ConstructionScript)