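; Key pickup platform for the maze game that lets the player collect a key by pressing Interact.
; Overlapping the trigger volume enables the player's input on the actor and shows a pickup prompt through the Gm_Maze HUD; leaving disables input and clears the message.
; Interacting destroys the Key component, increments the character's key count, refreshes the HUD skull display and plays a pickup sound at the player.
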(event OnComponentBeginOverlap(TriggerVolume)
  (params (OverlappedComponent :type Primitive%20Component%20Object%20Reference) (OtherActor :type Actor%20Object%20Reference) (OtherComp :type Primitive%20Component%20Object%20Reference) (OtherBodyIndex :type Integer) (bFromSweep :type Boolean) (SweepResult :type Hit%20Result%20Structure%20%28by%20ref%29))
  (if (== OtherActor (Game|GetPlayerCharacter 0))
    (Input|EnableInput (Game|GetPlayerController 0))
    (bind _asgm_maze (Utilities|Casting|CastToGm_Maze (Game|GetGameMode)))
    (Utilities|IsValid (Variables|Default|GetKey)
      (:Is%20Valid
        (Variables|/Game/UI/WB_HeadsUpDisplay.WB_HeadsUpDisplay_C|SetMessage (Variables|/Game/Game/Game/GM_Maze.Gm_Maze_C|GetHeadsUpDisplay _asgm_maze) "Press E to PickUp Key")
        (Default|UpdateMessage (Variables|/Game/Game/Game/GM_Maze.Gm_Maze_C|GetHeadsUpDisplay _asgm_maze))))))

(event OnComponentEndOverlap(TriggerVolume)
  (params (OverlappedComponent :type Primitive%20Component%20Object%20Reference) (OtherActor :type Actor%20Object%20Reference) (OtherComp :type Primitive%20Component%20Object%20Reference) (OtherBodyIndex :type Integer))
  (if (== OtherActor (Game|GetPlayerCharacter 0))
    (Input|DisableInput (Game|GetPlayerController 0))
    (bind _asgm_maze (Utilities|Casting|CastToGm_Maze (Game|GetGameMode)))
    (Variables|/Game/UI/WB_HeadsUpDisplay.WB_HeadsUpDisplay_C|SetMessage (Variables|/Game/Game/Game/GM_Maze.Gm_Maze_C|GetHeadsUpDisplay _asgm_maze) "")
    (Default|UpdateMessage (Variables|/Game/Game/Game/GM_Maze.Gm_Maze_C|GetHeadsUpDisplay _asgm_maze))))

(event Input|ActionEvents|InputActionInteract
  (params (Key :type Key%20Structure))
  (:Pressed
    (Utilities|IsValid (Variables|Default|GetKey)
      (:Is%20Valid
        (Components|DestroyComponent (Variables|Default|GetKey))
        (bind _asplayer_character_bp (Utilities|Casting|CastToPlayer_Character_BP (Game|GetPlayerCharacter 0)))
        (Math|Integer|IncrementInt (Variables|/Game/Game/Player_Character_BP.Player_Character_BP_C|GetNumber%20of%20Keys _asplayer_character_bp)
          (:%20%20
            (bind _asgm_maze (Utilities|Casting|CastToGm_Maze (Game|GetGameMode)))
            (Default|UpdateSkulls (Variables|/Game/Game/Game/GM_Maze.Gm_Maze_C|GetHeadsUpDisplay _asgm_maze))
            (Audio|PlaySoundatLocation "/Game/Sounds/PickupSkull_SFX.PickupSkull_SFX" (Transformation|GetActorLocation (Game|GetPlayerCharacter 0)) "0, 0, 0" 1.0 1.0 0.0 0 0 0)))))))

(fn ConstructionScript)